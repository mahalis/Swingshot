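; Game mode for the swing game that runs the title, options and pause screens, music, settings and target spawning.
; BeginPlay builds the menus; UI mode switches input, cursor, HUD and view between menu camera and pawn.
; Once play begins, a looping timer adds random batches of targets up to a cap.
; Each target uses best-candidate sampling: the random, curve-warped point in the spawn volume farthest from existing targets wins.
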(event EventBeginPlay
  (Utilities|FlowControl|Sequence
    (:then_0
      (bind _outactors (Actor|GetAllActorsOfClass "/Game/Blueprints/Game/TargetSpawnVolume.TargetSpawnVolume_C"))
      (if (> (Utilities|Array|Length _outactors) 0)
        (Variables|Default|SetSpawnVolume (Utilities|Array|Get(acopy) _outactors))))
    (:then_1
      (Development|ExecuteConsoleCommand "r.TemporalAACurrentFrameWeight 0.4" 0))
    (:then_2
      (bind _outactors_2 (Actor|GetAllActorsOfClasswithTag "/Script/Engine.CameraActor" "MenuCamera"))
      (Variables|Default|SetTitleCamera (Utilities|Array|Get(acopy) _outactors_2)))
    (:then_3
      (bind _returnvalue (UserInterface|CreateWidget "/Game/Blueprints/UI/TitleScreenWidget.TitleScreenWidget_C"))
      (bind _output_get (Variables|Default|SetTitleScreen _returnvalue))
      (UserInterface|Viewport|AddtoViewport _output_get 1)
      (bind _returnvalue_2 (UserInterface|CreateWidget "/Game/Blueprints/UI/OptionsWidget.OptionsWidget_C"))
      (bind _output_get_2 (Variables|Default|SetOptionsScreen _returnvalue_2))
      (UserInterface|Viewport|AddtoViewport _output_get_2 2)
      (bind _returnvalue_3 (UserInterface|CreateWidget "/Game/Blueprints/UI/PauseScreenWidget.PauseScreenWidget_C"))
      (bind _output_get_3 (Variables|Default|SetPauseScreen _returnvalue_3))
      (UserInterface|Viewport|AddtoViewport _output_get_3 1)
      (Widget|SetVisibility _output_get_3 "Hidden"))
    (:then_4
      (CallFunction|ShowTitleScreen))
    (:then_5
      (bind _returnvalue_4 (Audio|SpawnSound2D "/Game/Sounds/Lights.Lights" 1.0 1.0 0.0 0))
      (Variables|Default|SetMusic _returnvalue_4))
    (:then_6
      (CallFunction|SetSettings))))

(fn ConstructionScript)

(fn AddTarget
  (params (Existing :type Array%20of%20Target%20Object%20References))
  (bind _candidatelocations (LocalVariables|GetCandidateLocations))
  (Utilities|IsValid (Variables|Default|GetSpawnVolume)
    (:Is%20Valid
      (if (< (Utilities|Array|Length Existing) (Variables|Default|GetMaximumTargetCount)) ; cap the number of targets
        (LocalVariables|SetStuffToAvoid Existing)
        (for _index (range 0 20)
          (bind _location (CallFunction|FindCandidateTargetLocation))
          (bind _returnvalue (Utilities|Array|Add _candidatelocations _location))
          ;[1 1 1] find the closest distance for this candidate point to any of the stuff we're avoiding
          (LocalVariables|SetClosestDistanceToAvoidingStuff 9e+06)
          (for _array_element (LocalVariables|GetStuffToAvoid)
            (LocalVariables|SetClosestDistanceToAvoidingStuff (Math|Float|Min(Float) (Class|KismetMathLibrary|VectorDistanceSquared (Transformation|GetActorLocation _array_element) (Utilities|Array|Get(acopy) _candidatelocations _returnvalue)) (LocalVariables|GetClosestDistanceToAvoidingStuff))))
          (Utilities|Array|Add (LocalVariables|GetCandidateSquaredDistances) (LocalVariables|GetClosestDistanceToAvoidingStuff)))
        (bind _returnvalue_2 (Game|SpawnActorfromClass "/Game/Blueprints/World/Target.Target_C" (Math|Transform|MakeTransform (Utilities|Array|Get(acopy) (LocalVariables|GetCandidateLocations) (.IndexOfMaxValue (Math|Float|MaxOfFloatArray (LocalVariables|GetCandidateSquaredDistances)))) "0, 0, 0" "1,1,1") "AdjustIfPossibleButAlwaysSpawn" 0 0))
        (return _returnvalue_2)))))

(fn FindCandidateTargetLocation
  (bind _spawnvolume (Variables|Default|GetSpawnVolume))
  (bind _box (Variables|/Game/Blueprints/Game/TargetSpawnVolume.TargetSpawnVolume_C|GetBox _spawnvolume))
  (bind _returnvalue (Components|Box|GetUnscaledBoxExtent _box))
  (bind _output_get (LocalVariables|SetOriginalRandomPoint (Math|Random|RandomPointinBoundingBox "0, 0, 0" _returnvalue)))
  (return (Math|Transform|TransformLocation (Transformation|GetWorldTransform _box) (Math|Vector|MakeVector (.X (Math|Vector|BreakVector _output_get)) (* (.Y (Math|Vector|BreakVector _output_get)) (+ 1.0 (* (- 1.0 (Math|Float|Power (/ (.X (Math|Vector|BreakVector _output_get)) (* (.X (Math|Vector|BreakVector _returnvalue)) 0.5)) 2.0)) 0.5))) (.Z (Math|Vector|BreakVector _output_get))))))

(fn ConsiderAddingNewTargets
  (bind _outactors (Actor|GetAllActorsOfClass "/Game/Blueprints/World/Target.Target_C"))
  (bind _output_get (LocalVariables|SetTargets _outactors))
  (if (> (- (Variables|Default|GetMaximumTargetCount) (Utilities|Array|Length _output_get)) 0)
    (for _index (range 0 (Math|Random|RandomIntegerinRange 0 (Math|Integer|Min(Integer) (- (Variables|Default|GetMaximumTargetCount) (Utilities|Array|Length _output_get)) 4)))
      (bind _result (CallFunction|AddTarget (LocalVariables|GetTargets)))
      (Utilities|IsValid _result
        (:Is%20Valid
          (Utilities|Array|Add (LocalVariables|GetTargets) _result))))))

(fn BeginGame
  (Utilities|FlowControl|Sequence
    (:then_0
      (CallFunction|ConsiderAddingNewTargets))
    (:then_1
      (Utilities|Time|SetTimerbyFunctionName 0 "ConsiderAddingNewTargets" 4.0 true))
    (:then_2
      (Widget|SetVisibility (Variables|Default|GetTitleScreen) "Hidden"))
    (:then_3
      (CallFunction|SetUIMode false))
    (:then_4
      (Variables|Default|SetInGame true))))

(fn ShowTitleScreen
  (bind _titlescreen (Variables|Default|GetTitleScreen))
  (Widget|SetVisibility _titlescreen "Visible")
  (Widget|SetVisibility (Variables|Default|GetOptionsScreen) "Hidden")
  (CallFunction|SetUIMode true _titlescreen))

(fn SetUIMode
  (params (UI :type Boolean) (InitialFocusWidget :type Widget%20Object%20Reference))
  (bind _returnvalue (Game|GetPlayerController 0))
  (bind _returnvalue_2 (Game|Player|GetPlayerPawn 0))
  (if UI
    (Input|SetInputModeUIOnly _returnvalue InitialFocusWidget "DoNotLock")
    (Widget|SetKeyboardFocus InitialFocusWidget)
    (else
      (Input|SetInputModeGameOnly (Game|GetPlayerController 0))
      (Class|GameplayStatics|SetViewportMouseCaptureMode "CapturePermanently_IncludingInitialMouseDown")))
  (Variables|/Script/Engine.PlayerController|SetbShowMouseCursor _returnvalue UI)
  (Game|Player|SetViewTargetwithBlend _returnvalue (select UI (Variables|Default|GetTitleCamera) _returnvalue_2) 0.0 "VTBlend_Linear" 0.0 false)
  (bind _asswing_pawn (Utilities|Casting|CastToSwingPawn _returnvalue_2))
  (Utilities|IsValid (Variables|/Game/Blueprints/Player/SwingPawn.SwingPawn_C|GetHUD _asswing_pawn)
    (:Is%20Valid
      (Widget|SetVisibility (Variables|/Game/Blueprints/Player/SwingPawn.SwingPawn_C|GetHUD _asswing_pawn) (select UI "Hidden" "Visible")))))

(fn ShowOptionsScreen
  (bind _optionsscreen (Variables|Default|GetOptionsScreen))
  (Widget|SetVisibility (Variables|Default|GetTitleScreen) "Hidden")
  (Widget|SetVisibility (Variables|Default|GetPauseScreen) "Hidden")
  (Widget|SetVisibility _optionsscreen "Visible")
  (Widget|SetFocus _optionsscreen))

(fn HideOptionsScreen
  (bind _titlescreen (Variables|Default|GetTitleScreen))
  (bind _ingame (Variables|Default|GetInGame))
  (bind _pausescreen (Variables|Default|GetPauseScreen))
  (bind _returnvalue (select _ingame _pausescreen _titlescreen))
  (Widget|SetVisibility (Variables|Default|GetOptionsScreen) "Hidden")
  (Widget|SetVisibility _returnvalue "Visible")
  (Widget|SetKeyboardFocus _returnvalue))

(fn SetPaused
  (params (Is :type Boolean))
  (bind _pausescreen (Variables|Default|GetPauseScreen))
  (Game|SetGamePaused Is)
  (Widget|SetVisibility _pausescreen (select Is "Visible" "Hidden"))
  (CallFunction|SetUIMode Is _pausescreen))

(fn GetSettings
  (return (Variables|Default|GetSettings)))

(fn SetSettings
  (params (New :type Game%20Settings%20Structure))
  (LocalVariables|SetPrevious (Variables|Default|GetSettings))
  (bind _output_get (Variables|Default|SetSettings New))
  (Utilities|FlowControl|Sequence
    (:then_0
      (Audio|Components|Audio|SetVolumeMultiplier (Variables|Default|GetMusic) (* (.musicvolume _output_get) 0.1) :!class /Script/Engine.AudioComponent))
    (:then_1
      (Class|AutomationBlueprintFunctionLibrary|SetScalabilityQualityLevelRelativetoMax (Utilities|Select :Index (.graphicslevel _output_get) :Option%200 3 :Option%201 2 :Option%202 1)))
    (:then_2
      (Development|ExecuteConsoleCommand (Utilities|String|BuildString(Integer) "" "r.RayTracing.Reflections " (Math|Integer|SelectInt 1 0 (.raytracing _output_get))) (Game|GetPlayerController 0)))))

(fn SoundVolumeMultiplier
  (return (* (.soundvolume (Variables|Default|GetSettings)) 0.2)))