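; Target is a one-shot bubble pickup in the world that another actor can acquire, bursting on acquisition.
; The construction script scales the bubble mesh to match the collision sphere's radius.
; ConsiderAcquisition rejects repeat calls, then hides the bubble, disables collision and fires a burst particle system fed the acquirer's velocity.
; It reports success and destroys the actor after a short timer delay.
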(event EventBeginPlay)

(event Collision|EventActorBeginOverlap
  (params (OtherActor :type Actor%20Object%20Reference)))

(event EventTick
  (params (DeltaSeconds :type Float%20%28single-precision%29)))

(fn ConstructionScript
  (Transformation|SetRelativeScale3D (Variables|Default|GetBubbleMesh) (Math|Conversions|ToVector(Float) (* (Variables|/Script/Engine.SphereComponent|GetSphereRadius (Variables|Default|GetSphere)) 0.012))))

(fn ConsiderAcquisition
  (params (By :type Swing%20Pawn%20Object%20Reference))
  (bind _burstsystem (Variables|Default|GetBurstSystem))
  (if (Variables|Default|GetHasBeenAcquired)
    (return false)
    (else
      (Utilities|FlowControl|Sequence
        (:then_0
          (Variables|Default|SetHasBeenAcquired true))
        (:then_1
          (Rendering|SetVisibility (Variables|Default|GetBubbleMesh) false false))
        (:then_2
          (Collision|SetCollisionEnabled (Variables|Default|GetSphere) "NoCollision"))
        (:then_3
          (Utilities|Time|SetTimerbyFunctionName 0 "CleanUp" 3.0))
        (:then_4
          (Effects|Components|ParticleSystem|SetVectorParameter _burstsystem "IncomingVelocity" (Transformation|GetVelocity By))
          (Components|Activation|Activate _burstsystem false))
        (:then_5
          (return true))))))

(fn CleanUp
  (Actor|DestroyActor))