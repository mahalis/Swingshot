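; Player pawn for a first-person-style grapple-swinging game, with air jumps, target pickups and a HUD.
; Each tick it picks the best cached Hook by view alignment and distance, then attaches on input with a launch impulse and beam.
; A fixed 60 Hz timer applies a clamped spring pull that damps sideways velocity; the rope-force variant is unused.
; Falling below a height floor triggers a force-field bounce that restores the air jump.
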(event EventBeginPlay
  (Utilities|FlowControl|Sequence
    (:then_0
      (Setup|FindAllHooks))
    (:then_1
      (bind _returnvalue (UserInterface|CreateWidget "/Game/Blueprints/UI/HUDWidget.HUDWidget_C" (Game|GetPlayerController 0)))
      (bind _output_get (Variables|Default|SetHUD _returnvalue))
      (UserInterface|Viewport|AddtoViewport _output_get 0))
    (:then_2
      (Utilities|Time|SetTimerbyFunctionName 0 "ApplyForces" 0.016667 true))))

(event Collision|EventActorBeginOverlap
  (params (OtherActor :type Actor%20Object%20Reference))
  (bind _astarget (Utilities|Casting|CastToTarget OtherActor))
  (bind _newlyacquired (Default|ConsiderAcquisition _astarget self))
  (if _newlyacquired
    (CallFunction|HandleTargetAcquisition)))

(event EventTick
  (params (DeltaSeconds :type Float%20%28single-precision%29))
  (HookTargeting|LookforHooks)
  (CallFunction|ConsiderAttaching)
  (Forces|ApplyBounceifNeeded)
  (CallFunction|UpdateToolActivity DeltaSeconds))

(event EventOnJumped
  (Variables|Default|SetHasJump false))

(event EventOnLanded
  (params (Hit :type Hit%20Result%20Structure%20%28by%20ref%29))
  (Variables|Default|SetHasJump true))

(event Input|ActionEvents|InputActionJump
  (params (Key :type Key%20Structure :default "None"))
  (:Pressed
    (CallFunction|DoJumporAirJump)
    (Utilities|IsValid (Variables|HookTargeting|GetAttachedHook)
      (:Is%20Valid
        (CallFunction|Detach))))
  (:Released
    (Character|StopJumping)))

(event Input|ActionEvents|InputActionAttach
  (params (Key :type Key%20Structure :default "None"))
  (:Pressed
    (Variables|HookTargeting|SetWantsAttach true))
  (:Released
    (Variables|HookTargeting|SetWantsAttach false)
    (Utilities|IsValid (Variables|HookTargeting|GetAttachedHook)
      (:Is%20Valid
        (if (> (Utilities|Time|GetGameTimeinSeconds) (+ (Variables|HookTargeting|GetLastAttachTime) 1.0))
          (CallFunction|Detach)
          (CallFunction|PlayReleaseSound))))))

(event Input|AxisEvents|InputAxisPanRate
  (params (AxisValue :type Float%20%28single-precision%29))
  ;[1 1 1] camera controls
  (Pawn|Input|AddControllerYawInput (* AxisValue (Utilities|Time|GetWorldDeltaSeconds) 7e+01)))

(event Input|AxisEvents|InputAxisPan
  (params (AxisValue :type Float%20%28single-precision%29))
  ;[1 1 1] camera controls
  (Pawn|Input|AddControllerYawInput (* AxisValue 0.8)))

(event Input|AxisEvents|InputAxisMoveForward
  (params (AxisValue :type Float%20%28single-precision%29))
  (Class|PawnMovementComponent|AddInputVector (Variables|Character|GetCharacterMovement) (* (Transformation|GetActorForwardVector) AxisValue) false))

(event Input|AxisEvents|InputAxisTiltRate
  (params (AxisValue :type Float%20%28single-precision%29))
  ;[1 1 1] camera controls
  (Pawn|Input|AddControllerPitchInput (* AxisValue (Utilities|Time|GetWorldDeltaSeconds) 7e+01)))

(event Input|AxisEvents|InputAxisTilt
  (params (AxisValue :type Float%20%28single-precision%29))
  ;[1 1 1] camera controls
  (Pawn|Input|AddControllerPitchInput (* AxisValue -0.8)))

(event Input|AxisEvents|InputAxisMoveRight
  (params (AxisValue :type Float%20%28single-precision%29))
  (Class|PawnMovementComponent|AddInputVector (Variables|Character|GetCharacterMovement) (* (Transformation|GetActorRightVector) AxisValue) false))

(event Input|KeyboardEvents|Escape
  (params (Key :type Key%20Structure :default "None"))
  (:Pressed
    (bind _asswing_mode (Utilities|Casting|CastToSwingMode (Game|GetGameMode)))
    (Default|SetPaused _asswing_mode true)))

(fn ConstructionScript)

(fn FindAllHooks
  (Utilities|Array|Clear (Variables|Setup|GetKnownHooks))
  (bind _outactors (Actor|GetAllActorsOfClass "/Game/Blueprints/World/Hook.Hook_C"))
  (for _array_element _outactors
    (Utilities|Array|Add (Variables|Setup|GetKnownHooks) _array_element)))

(fn FindLookingHook
  (for (_array_element _array_index) (Variables|Setup|GetKnownHooks)
    (bind (_lookingness _distance) (HookTargeting|EvaluateHookCandidacy _array_element))
    (if (Math|Boolean|ANDBoolean (> _lookingness (Math|Trig|Sin(Degrees) 7e+01)) (< _distance 3e+03) (> (CallFunction|WeightTarget _lookingness _distance) (CallFunction|WeightTarget (LocalVariables|GetBestCandidateLookingness) (LocalVariables|GetBestCandidateDistance))))
      (LocalVariables|SetBestCandidateIndex _array_index)
      (LocalVariables|SetBestCandidateLookingness _lookingness)
      (LocalVariables|SetBestCandidateDistance _distance)))
  (if (>= (LocalVariables|GetBestCandidateIndex) 0)
    (return (Utilities|Array|Get(acopy) (Variables|Setup|GetKnownHooks) (LocalVariables|GetBestCandidateIndex)))
    (else
      (return 0))))

(fn EvaluateHookCandidacy
  (params (Hook :type Hook%20Object%20Reference))
  (bind (_outlocation _outrotation) (Actor|GetActorEyesViewPoint))
  (bind _returnvalue (Math|Vector|MakeVector 1.0 1.0 0.5))
  (bind _output_get (LocalVariables|SetOffset (- (Transformation|GetActorLocation Hook) _outlocation)))
  (return (Math|Vector|DotProduct (Math|Vector|Normalize (* (/ _output_get (Math|Vector|VectorLength _output_get)) _returnvalue)) (Math|Vector|Normalize (* (Math|Vector|GetForwardVector _outrotation) _returnvalue))) (Math|Vector|VectorLength _output_get)))

(fn SetTargetedHook
  (params (New :type Hook%20Object%20Reference))
  (if (!= New (Variables|HookTargeting|GetTargetedHook)) ; don't do anything if the target hasn't changed
    (Utilities|IsValid (Variables|HookTargeting|GetTargetedHook)
      (:Is%20Valid
        (Default|SetIsTargeted (Variables|HookTargeting|GetTargetedHook) false))
      (:Is%20Not%20Valid
        _))
    (Utilities|IsValid New
      (:Is%20Valid
        (Default|SetIsTargeted New true))
      (:Is%20Not%20Valid
        _))
    (Variables|HookTargeting|SetTargetedHook New)))

(fn LookforHooks
  (bind _best (HookTargeting|FindLookingHook)) ; may want to move this to a timer instead of a tick, or decrease the pawn's tick frequency
  (HookTargeting|SetTargetedHook _best))

(fn ConsiderAttaching
  (bind _targetedhook (Variables|HookTargeting|GetTargetedHook))
  (bind _attachmentbeamsystem (Variables|Default|GetAttachmentBeamSystem))
  (bind _targetedhook_2 (Variables|HookTargeting|GetTargetedHook))
  (Utilities|IsValid (Variables|HookTargeting|GetAttachedHook) ; are we currently attached
    (:Is%20Valid
      (if (and (Utilities|IsValid _targetedhook) (!= _targetedhook (Variables|HookTargeting|GetAttachedHook))) ; is the target a different hook
        (if (and (Variables|HookTargeting|GetWantsAttach) (Utilities|IsValid _targetedhook_2)) :!label _label
          (Utilities|IsValid (Variables|HookTargeting|GetAttachedHook)
            (:Is%20Valid
              (CallFunction|Detach))
            (:Is%20Not%20Valid
              _))
          (Utilities|FlowControl|Sequence
            (:then_0
              (Variables|HookTargeting|SetAttachedHook _targetedhook_2))
            (:then_1
              (Default|SetIsHooked _targetedhook_2 true))
            (:then_2
              (Variables|HookTargeting|SetWantsAttach false))
            (:then_3
              (Variables|HookTargeting|SetLastAttachTime (Utilities|Time|GetGameTimeinSeconds)))
            (:then_4
              (Components|Activation|Activate _attachmentbeamsystem true)
              (Niagara|SetNiagaraVariable(Vector3) _attachmentbeamsystem "EndLocation" (Transformation|GetActorLocation (Variables|HookTargeting|GetAttachedHook))))
            (:then_5
              (CallFunction|ApplyInitialAttachmentImpulse))
            (:then_6
              (Audio|PlaySound2D "/Game/Sounds/Grapple6.Grapple6" 1.0 1.0 0.0 0 0))
            (:then_7
              (Variables|Default|SetHasJump true))))))
    (:Is%20Not%20Valid
      (goto _label))))

(fn ConsiderApplyingAttachmentForce
  (bind _returnvalue (Transformation|GetActorLocation))
  (bind _attachedhook (Variables|HookTargeting|GetAttachedHook))
  (bind _returnvalue_2 (Transformation|GetActorLocation _attachedhook))
  (bind _returnvalue_3 (- _returnvalue_2 _returnvalue))
  (Utilities|IsValid _attachedhook
    (:Is%20Valid
      (bind _output_get (LocalVariables|SetHookDistance (Math|Vector|VectorLength _returnvalue_3)))
      (LocalVariables|SetHookDirection (/ _returnvalue_3 _output_get))
      (Pawn|Components|CharacterMovement|SetMovementMode (Variables|Character|GetCharacterMovement) "MOVE_Falling" 0)
      (Forces|ApplySpringAttachmentForce (LocalVariables|GetHookDirection) (LocalVariables|GetHookDistance)))))

(fn Detach
  (Utilities|IsValid (Variables|HookTargeting|GetAttachedHook)
    (:Is%20Valid
      (Default|SetIsHooked (Variables|HookTargeting|GetAttachedHook) false)
      (Variables|HookTargeting|SetAttachedHook 0)
      (Components|Activation|Deactivate (Variables|Default|GetAttachmentBeamSystem)))))

(fn ApplySpringAttachmentForce
  (params (Direction :type Vector) (Distance :type Float%20%28single-precision%29))
  (bind (_x _y) (Math|Vector|BreakVector Direction))
  (bind _returnvalue (Math|Float|Clamp(Float) Distance 5e+02 1.2e+03))
  (bind _returnvalue_2 (- 0.0 _y))
  (bind _returnvalue_3 (* _returnvalue 8e+02))
  (bind _returnvalue_4 (Math|Vector|MakeVector _returnvalue_2 _x 0.0))
  (bind _returnvalue_5 (* Direction _returnvalue_3))
  (Physics|AddForce (Variables|Character|GetCharacterMovement) (- (* _returnvalue_5 (Math|Vector|SelectVector "1.000000,1.000000,0.800000" "1.000000,1.000000,1.600000" (> (.Z (Math|Vector|BreakVector _returnvalue_5)) 0.0))) (* _returnvalue_4 (* (Math|Vector|DotProduct _returnvalue_4 (Variables|/Script/Engine.MovementComponent|GetVelocity (Variables|Character|GetCharacterMovement))) 0.8)))))

(fn ApplyRopeAttachmentForce
  (params (Direction :type Vector) (Distance :type Float%20%28single-precision%29))
  (bind _charactermovement (Variables|Character|GetCharacterMovement))
  (bind _velocity (Variables|/Script/Engine.MovementComponent|GetVelocity _charactermovement))
  (if (> Distance 2.8e+02)
    (Physics|AddImpulse _charactermovement (* (* (* Direction (/ (Math|Vector|VectorLengthSquared (- _velocity (Math|Vector|ProjectVectorontoVector _velocity Direction))) Distance)) (Variables|/Script/Engine.CharacterMovementComponent|GetMass _charactermovement)) (Utilities|Time|GetWorldDeltaSeconds)) true)))

(fn CanJumpInternal
  (return (or (Utilities|IsValid (Variables|HookTargeting|GetAttachedHook)) (Variables|Default|GetHasJump))))

(fn ApplyForces
  (Forces|ConsiderApplyingAttachmentForce))

(fn EvaluateBounceState
  (return (/ (- (Utilities|Time|GetGameTimeinSeconds) (Variables|Forces|GetLastBounceTime)) (Variables|Forces|GetBounceDuration))))

(fn ApplyBounceifNeeded
  (bind _charactermovement (Variables|Character|GetCharacterMovement))
  (bind _progress (Forces|EvaluateBounceState))
  (if (Math|Float|InRange(Float) _progress 0.0 1.0)
    (Variables|/Script/Engine.MovementComponent|SetVelocity _charactermovement (Math|Vector|MakeVector (.x (Variables|/Script/Engine.MovementComponent|GetVelocity _charactermovement)) (.y (Variables|/Script/Engine.MovementComponent|GetVelocity _charactermovement)) (Math|Float|Lerp (Variables|Forces|GetBounceStartSpeed) (Math|Float|Max(Float) (* (Math|Float|Absolute(Float) (Variables|Forces|GetBounceStartSpeed)) 0.95) 9e+02) _progress)))
    (elif (< (.z (Transformation|GetActorLocation)) (Math|Float|MakeLiteralFloat -2e+02))
      (Variables|Forces|SetLastBounceTime (Utilities|Time|GetGameTimeinSeconds))
      (Variables|Forces|SetBounceStartSpeed (.z (Variables|/Script/Engine.MovementComponent|GetVelocity (Variables|Character|GetCharacterMovement))))
      (Audio|PlaySound2D "/Game/Sounds/ForceFieldBounce5.ForceFieldBounce5" 1.0 1.0 0.0 0 0)
      (Variables|Default|SetHasJump true))))

(fn HandleTargetAcquisition
  (bind _charactermovement (Variables|Character|GetCharacterMovement))
  (Variables|/Script/Engine.MovementComponent|SetVelocity _charactermovement (* (Variables|/Script/Engine.MovementComponent|GetVelocity _charactermovement) 0.8))
  (Default|Flash (Variables|Default|GetHUD)))

(fn ApplyInitialAttachmentImpulse
  (bind _output_get (LocalVariables|SetDirection (- (Transformation|GetActorLocation (Variables|HookTargeting|GetAttachedHook)) (Transformation|GetActorLocation))))
  (bind _output_get_2 (LocalVariables|SetBaselineSpeed (Math|Vector|VectorLength (* _output_get "1.000000,1.000000,2.000000"))))
  (if (< _output_get_2 (LocalVariables|GetMinimumSpeed))
    (LocalVariables|SetSpeedAdjustment (/ (LocalVariables|GetMinimumSpeed) (LocalVariables|GetBaselineSpeed)))
    (elif (> (LocalVariables|GetBaselineSpeed) (LocalVariables|GetMaximumSpeed))
      (bind _output_get_3 (LocalVariables|SetSpeedAdjustment (/ (LocalVariables|GetMaximumSpeed) (LocalVariables|GetBaselineSpeed))))))
  (Physics|AddImpulse (Variables|Character|GetCharacterMovement) (* (LocalVariables|GetDirection) (* _output_get_3 0.5)) true))

(fn UpdateToolActivity
  (params (DeltaTime :type Float%20%28single-precision%29))
  (bind _output_get (Variables|Default|SetCrystalRotation (Math|Float|%(Float) (+ (Variables|Default|GetCrystalRotation) (* (Math|Float|SelectFloat -2.4e+02 -2e+01 (Utilities|IsValid (Variables|HookTargeting|GetAttachedHook))) DeltaTime)) 3.6e+02)))
  (Transformation|SetRelativeRotation (Variables|Default|GetToolCrystal) (Math|Rotator|MakeRotator 0.0 _output_get 0.0) false false))

(fn WeightTarget
  (params (Lookingness :type Float%20%28single-precision%29) (Distance :type Float%20%28single-precision%29))
  (return (- Lookingness (/ Distance 6e+03))))

(fn PlayReleaseSound
  (Audio|PlaySound2D "/Game/Sounds/Release.Release" 1.0 1.0 0.0 0 0))

(fn DoJumporAirJump
  (bind _charactermovement (Variables|Character|GetCharacterMovement))
  (if (Utilities|Enum|Equal(Enum) (Variables|/Script/Engine.CharacterMovementComponent|GetMovementMode _charactermovement) "MOVE_Walking")
    (Character|Jump)
    (Audio|PlaySound2D "/Game/Sounds/Jump1.Jump1" 1.0 1.0 0.0 0 0 :!label _label)
    (elif (Variables|Default|GetHasJump)
      (Physics|AddImpulse _charactermovement (Math|Vector|MakeVector 0.0 0.0 (Variables|/Script/Engine.CharacterMovementComponent|GetJumpZVelocity _charactermovement)) true)
      (Variables|Default|SetHasJump false)
      (goto _label))))