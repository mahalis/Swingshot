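; Hook is a world actor that shows whether it is targeted or hooked through the shape of its cube.
; SetIsTargeted and SetIsHooked store their flags, then call UpdateState, which also runs at construction.
; UpdateState rescales the cube: being hooked narrows its width and depth, and being targeted makes it taller.
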(event EventBeginPlay)

(event Collision|EventActorBeginOverlap
  (params (OtherActor :type Actor%20Object%20Reference)))

(event EventTick
  (params (DeltaSeconds :type Float%20%28single-precision%29)))

(fn ConstructionScript
  (CallFunction|UpdateState))

(fn SetIsTargeted
  (params (Is :type Boolean))
  (Variables|Default|SetTargeted Is)
  (CallFunction|UpdateState))

(fn UpdateState
  (bind _hooked (Variables|Default|GetHooked))
  (bind _returnvalue (Math|Float|SelectFloat 0.2 0.5 _hooked))
  (Transformation|SetRelativeScale3D (Variables|Default|GetCube) (Math|Vector|MakeVector _returnvalue _returnvalue (Math|Float|SelectFloat 0.5 0.2 (Variables|Default|GetTargeted)))))

(fn SetIsHooked
  (params (Is :type Boolean))
  (Variables|Default|SetHooked Is)
  (CallFunction|UpdateState))